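; Turret actor that targets BP_EVIL_Sphere actors, shoots BP_Bullet at them and can be destroyed by them.
; DetectionRange overlap events set or clear the target, backed by a timer that picks an overlapping sphere when none is held.
; Tick smoothly rotates Body toward the target and drives a fire cooldown, clearing the target after each shot.
; A timed HurtBox check subtracts health per overlapping sphere and destroys the turret at zero.
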(event OnComponentBeginOverlap(DetectionRange)
  (params (OverlappedComponent :type Primitive%20Component%20Object%20Reference) (OtherActor :type Actor%20Object%20Reference) (OtherComp :type Primitive%20Component%20Object%20Reference) (OtherBodyIndex :type Integer) (bFromSweep :type Boolean) (SweepResult :type Hit%20Result%20Structure%20%28by%20ref%29))
  (bind _asbp_evil_sphere (Utilities|Casting|CastToBP_EVIL_Sphere OtherActor))
  (Variables|Default|SetCurrentTarget _asbp_evil_sphere))

(event OnComponentEndOverlap(DetectionRange)
  (params (OverlappedComponent :type Primitive%20Component%20Object%20Reference) (OtherActor :type Actor%20Object%20Reference) (OtherComp :type Primitive%20Component%20Object%20Reference) (OtherBodyIndex :type Integer))
  (if (== OtherActor (Variables|Default|GetCurrentTarget))
    (Variables|Default|SetCurrentTarget 0)))

(event EventBeginPlay
  (Utilities|FlowControl|Sequence
    (:then_0
      (|DetectEnemies))
    (:then_1
      (|TakeDamage))))

(fn ConstructionScript)

(event Custom|CheckHurtBox
  (Utilities|Array|ForEachLoopwithBreak (Collision|GetOverlappingActors (Variables|Default|GetHurtBox) "/Game/Blueprints/BP_EVIL_Sphere.BP_EVIL_Sphere_C" :!class /Script/Engine.PrimitiveComponent)
    (:LoopBody
      (Variables|Default|SetHealth (- (Variables|Default|GetHealth) 1))
      (if (<= (Variables|Default|GetHealth) 0)
        (Variables|Default|SetIsDead true)))
    (:Completed
      (if (Variables|Default|GetIsDead)
        (Actor|DestroyActor)
        (else
          (Utilities|Time|SetTimerbyEvent (delegate Custom|CheckHurtBox) 0.5 true))))))

(event Custom|CheckForTargets
  (Variables|Default|GetCurrentTarget
    (:then
      (Utilities|Time|SetTimerbyEvent (delegate Custom|CheckForTargets) 1.0 true))
    (:else
      (bind _asbp_evil_sphere (Utilities|Casting|CastToBP_EVIL_Sphere (Utilities|Array|Get(acopy) (Collision|GetOverlappingActors (Variables|Default|GetDetectionRange) "/Game/Blueprints/BP_EVIL_Sphere.BP_EVIL_Sphere_C" :!class /Script/Engine.PrimitiveComponent))))
      (Variables|Default|SetCurrentTarget _asbp_evil_sphere))))

(event EventTick
  (params (DeltaSeconds :type Float%20%28single-precision%29))
  (Utilities|IsValid (Variables|Default|GetCurrentTarget)
    (:Is%20Valid
      (return (Variables|Default|GetBody) (Math|Interpolation|RInterpTo (Transformation|GetWorldRotation (Variables|Default|GetBody)) (Math|Rotator|FindLookatRotation (Transformation|GetWorldLocation (Variables|Default|GetBody)) (Transformation|GetWorldLocation (Variables|/Script/Engine.Actor|GetRootComponent (|Inputs)))) DeltaSeconds 5.0)))))