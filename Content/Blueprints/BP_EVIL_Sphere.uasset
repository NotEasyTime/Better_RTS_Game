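; BP_EVIL_Sphere is an enemy that wanders in a straight line until it detects a base, then moves toward it.
; Tick nudges the capsule along world X by a fixed, unswept per-frame offset while Wander is set.
; The Detect overlap clears Wander and issues AIMoveTo to the base's CubeBody location.
; Bullets overlapping Sphere are destroyed and reduce Health; at zero it reports to WaveManagerRef and destroys itself.
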(event OnComponentBeginOverlap(Detect)
  (params (OverlappedComponent :type Primitive%20Component%20Object%20Reference) (OtherActor :type Actor%20Object%20Reference) (OtherComp :type Primitive%20Component%20Object%20Reference) (OtherBodyIndex :type Integer) (bFromSweep :type Boolean) (SweepResult :type Hit%20Result%20Structure%20%28by%20ref%29))
  (bind _asbp_base (Utilities|Casting|CastToBP_Base OtherActor))
  (Variables|Default|Setwander false)
  (AI|AIMoveTo self (Transformation|GetWorldLocation (Variables|/Game/Blueprints/BP_Base.BP_Base_C|GetCubeBody _asbp_base)) 0 5.0 false))

(event OnComponentBeginOverlap(Sphere)
  (params (OverlappedComponent :type Primitive%20Component%20Object%20Reference) (OtherActor :type Actor%20Object%20Reference) (OtherComp :type Primitive%20Component%20Object%20Reference) (OtherBodyIndex :type Integer) (bFromSweep :type Boolean) (SweepResult :type Hit%20Result%20Structure%20%28by%20ref%29))
  (bind _asbp_bullet (Utilities|Casting|CastToBP_Bullet OtherActor))
  (Actor|DestroyActor _asbp_bullet)
  (Variables|Default|SetHealth (- (Variables|Default|GetHealth) 1))
  (if (< (Variables|Default|GetHealth) 1)
    (CallFunction|Die)))

(event Custom|die
  (bind _wavemanagerref (Variables|Default|GetWaveManagerRef))
  (Utilities|IsValid _wavemanagerref
    (:Is%20Valid
      (Default|RegisterEnemyDeath _wavemanagerref self))
    (:Is%20Not%20Valid
      _))
  (Actor|DestroyActor))

(event EventTick
  (params (DeltaSeconds :type Float%20%28single-precision%29))
  (if (Variables|Default|Getwander)
    (Transformation|AddWorldOffset (Variables|Collision|GetCapsuleComponent) "2.000000,0.000000,0.000000" false false)))

(fn ConstructionScript)