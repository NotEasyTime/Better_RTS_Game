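; BP_CamActor is a camera rig actor that provides pan and zoom functions.
; Pan moves the actor along world X and Y from a 2D input, scaled by move speed and frame delta, keeping height fixed without sweeping.
; Zoom changes the spring arm length by input and zoom speed, clamped between minimum and maximum limits.
; The event graph holds no logic, so both functions rely on external callers.
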(event EventBeginPlay)

(event Collision|EventActorBeginOverlap
  (params (OtherActor :type Actor%20Object%20Reference)))

(event EventTick
  (params (DeltaSeconds :type Float%20%28single-precision%29)))

(fn ConstructionScript)

(fn Pan
  (params (MoveInput :type Vector%202D%20Structure))
  (bind _returnvalue (Transformation|GetActorLocation))
  (bind (_x _y) (Math|Vector2D|BreakVector2D MoveInput))
  (bind (_x_2 _y_2 _z) (Math|Vector|BreakVector _returnvalue))
  (Transformation|SetActorLocation (Math|Vector|MakeVector (+ (* (Variables|Default|GetMoveSpeed) (Utilities|Time|GetWorldDeltaSeconds) _x) _x_2) (+ _y_2 (* _y (Utilities|Time|GetWorldDeltaSeconds) (Variables|Default|GetMoveSpeed))) _z) false false))

(fn Zoom
  (params (ZoomInput :type Float%20%28double-precision%29))
  (Variables|/Script/Engine.SpringArmComponent|SetTargetArmLength (Variables|Default|GetSpringArm) (Math|Float|Clamp(Float) (- (Variables|/Script/Engine.SpringArmComponent|GetTargetArmLength (Variables|Default|GetSpringArm)) (* ZoomInput (Variables|Default|GetZoomSpeed))) (Variables|Default|GetMinZoom) (Variables|Default|GetMaxZoom))))