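; BP_Camera is a player-controlled camera that pans and zooms through Enhanced Input.
; BeginPlay adds the IMC_Camera mapping context to player 0.
; IA_CameraMove offsets the actor along its forward and right vectors, scaled by MoveSpeed and delta time, without collision sweep.
; IA_CameraZoom changes the spring arm length by ZoomSpeed within min and max limits, without delta-time scaling.
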(event Input|EnhancedActionEvents|EnhancedInputActionIA_CameraMove
  (params (ActionValue :type Vector%202D%20Structure) (ElapsedSeconds :type Float%20%28double-precision%29) (TriggeredSeconds :type Float%20%28double-precision%29) (InputAction :type Input%20Action%20Object%20Reference :default "/Game/TopDown/Input/Actions/IA_CameraMove.IA_CameraMove"))
  (bind (_x _y) (Math|Vector2D|BreakVector2D ActionValue))
  (:Triggered
    (Transformation|SetActorLocation (+ (Transformation|GetActorLocation) (+ (* (Utilities|Time|GetWorldDeltaSeconds) (* (Variables|Default|GetMoveSpeed) (* (Transformation|GetActorRightVector) _x))) (* (* (* _y (Transformation|GetActorForwardVector)) (Variables|Default|GetMoveSpeed)) (Utilities|Time|GetWorldDeltaSeconds)))) false false)))

(event Input|EnhancedActionEvents|EnhancedInputActionIA_CameraZoom
  (params (ActionValue :type Float%20%28double-precision%29) (ElapsedSeconds :type Float%20%28double-precision%29) (TriggeredSeconds :type Float%20%28double-precision%29) (InputAction :type Input%20Action%20Object%20Reference :default "/Game/TopDown/Input/Actions/IA_CameraZoom.IA_CameraZoom"))
  (:Triggered
    (Variables|/Script/Engine.SpringArmComponent|SetTargetArmLength (Variables|Default|GetSpringArm) (Math|Float|Clamp(Float) (- (Variables|/Script/Engine.SpringArmComponent|GetTargetArmLength (Variables|Default|GetSpringArm)) (* ActionValue (Variables|Default|GetZoomSpeed))) (Variables|Default|GetMinZoom) (Variables|Default|GetMaxZoom)))))

(event EventBeginPlay
  (Input|AddMappingContext (PlayerController|LocalPlayerSubsystems|GetEnhancedInputLocalPlayerSubsystem (Game|GetPlayerController 0)) "/Game/TopDown/Input/IMC_Camera.IMC_Camera" 0 "(bIgnoreAllPressedKeysUntilRelease=True,bForceImmediately=False,bNotifyUserSettings=False)"))

(fn ConstructionScript)