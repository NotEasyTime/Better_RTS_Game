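; BP_SpawnManager runs endless, escalating waves of BP_EVIL_Sphere enemies.
; On BeginPlay it gathers every BP_SpawnPoint in the level, then starts a self-calling delayed loop that spawns one enemy per second at a random point.
; Once the spawn count exceeds the wave limit, it increments the wave counter, grows the limit, pauses briefly and restarts the loop.
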(event Custom|Spawn%20Enemy%20loop
  (Game|SpawnActorfromClass "/Game/Blueprints/BP_EVIL_Sphere.BP_EVIL_Sphere_C" (Transformation|GetWorldTransform (Variables|/Game/Blueprints/BP_SpawnPoint.BP_SpawnPoint_C|GetDefaultSceneRoot (Utilities|Array|Get(acopy) (Variables|Default|GetSpawnPoints) (Math|Integer|%(Integer) (Math|Random|RandomInteger 200) (Utilities|Array|Length (Variables|Default|GetSpawnPoints)))))) "Undefined" "MultiplyWithRoot" 0 0)
  (bind _output_get (Variables|Default|SetAmmountSpawn (+ (Variables|Default|GetAmmountSpawn) 1)))
  (if (> _output_get (Variables|Default|GetMaxSpawn))
    (Variables|Default|SetWaveCount (+ (Variables|Default|GetWaveCount) 1))
    (CallFunction|NextWave)
    (else
      (Utilities|FlowControl|Delay 1.0)
      (CallFunction|SpawnEnemyLoop))))

(event Custom|Next%20Wave
  (Variables|Default|SetAmmountSpawn 0)
  (Variables|Default|SetMaxSpawn (+ (* (Variables|Default|GetMaxSpawn) 2) 10))
  (Utilities|FlowControl|Delay 5.0)
  (Development|PrintString "Spawn Next Wave")
  (CallFunction|SpawnEnemyLoop))

(event EventBeginPlay
  (bind _outactors (Actor|GetAllActorsOfClass "/Game/Blueprints/BP_SpawnPoint.BP_SpawnPoint_C"))
  (Variables|Default|SetSpawnPoints _outactors)
  (CallFunction|SpawnEnemyLoop))

(event Collision|EventActorBeginOverlap
  (params (OtherActor :type Actor%20Object%20Reference)))

(event EventTick
  (params (DeltaSeconds :type Float%20%28single-precision%29)))

(fn ConstructionScript)